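; BP_QA_Controller automates QA screenshot capture from every BP_QA_Camera_Single placed in the level.
; On BeginPlay it gathers those cameras and starts a recursive CaptureScreenshots event.
; Each pass switches player 0's view target to the next camera, waits, and takes a 1080p high-res screenshot named from the export path, camera name and index, then repeats.
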(event `self.ReceiveBeginPlay`
  (bind _outactors (`GameplayStatics.GetAllActorsOfClass` "/QA_Tools/01_Blueprints/BP_QA_Camera_Single.BP_QA_Camera_Single_C"))
  (set `self.QA Cameras` _outactors)
  (`self.Capture Screenshots`))

(event `Capture Screenshots`
  (bind _counter (`self.counter`))
  (bind _output (`|GetArrayItem` (`self.QA Cameras`) _counter))
  (if (< (`self.counter`) (`KismetArrayLibrary.Array_Length` (`self.QA Cameras`)))
    (`PlayerController.SetViewTargetWithBlend` (`GameplayStatics.GetPlayerController` 0) _output 0.0 "VTBlend_Linear" 0.0 false)
    (`KismetSystemLibrary.Delay` (`self.Delay`))
    (`AutomationBlueprintFunctionLibrary.TakeHighResScreenshot` 1920 1080 (`KismetStringLibrary.Concat_StrStr` (`self.Export Path`) (`KismetSystemLibrary.GetDisplayName` _output) "#" (`KismetStringLibrary.Conv_IntToString` _counter)) null false false "Low" "" (`self.Delay`))
    (`KismetSystemLibrary.Delay` (`self.Delay`))
    (`/Engine/EditorBlueprintResources/StandardMacros.IncrementInt` (`self.counter`)
      (:`  `
        (`self.Capture Screenshots`)))))

(fn `UserConstructionScript`)